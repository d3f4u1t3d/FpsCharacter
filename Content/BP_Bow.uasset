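; BP_Bow is a bow weapon that spawns, charges and fires BP_Arrow projectiles.
; Reload spawns an arrow and attaches it to a socket on the bow mesh.
; While an arrow is valid, a timeline drives ChargeAmount, playing on BeginCharge and reversing on EndCharge.
; Fire detaches the arrow, passes it the charge, clears the reference, then stops and resets the timeline.
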(event `BeginCharge`
  (`self.Arrow`
    (:`then`
      (bind (_direction _chargeamount) (`Timeline|ChargeTimeline` :!label _label)
        (:`Update`
          (set `self.ChargeAmount` _chargeamount))))
    (:`else`)))

(event `StopCharge`
  (`|ExecutionSequence`
    (:`then_0`
      (goto _label :!via `Stop`))
    (:`then_1`
      (goto _label :!via `SetNewTime`))))

(event `EndCharge`
  (`self.Arrow`
    (:`then`
      (goto _label :!via `Reverse`))
    (:`else`)))

(event `Fire`
  (bind _arrow (`self.Arrow`)
    (:`then`
      (`self.K2_DetachFromActor` _arrow "KeepWorld" "KeepWorld" "KeepWorld")
      (`/Game/BP_Arrow.Fire` (`self.Arrow`) (`self.ChargeAmount`))
      (set `self.Arrow` null)
      (`self.StopCharge`))
    (:`else`)))

(event `Reload`
  (bind _returnvalue (`|SpawnActorFromClass` "/Game/BP_Arrow.BP_Arrow_C" (`KismetMathLibrary.MakeTransform` (0.0 0.0 0.0)) "Undefined" "OverrideRootScale" null "NewEnumerator2" null))
  (bind _output_get (set `self.Arrow` _returnvalue))
  (`self.K2_AttachToComponent` _output_get (`self.BowMesh`) "Arrow_Atach_Socket" "SnapToTarget" "SnapToTarget" "KeepWorld" true))

(fn `UserConstructionScript`)